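; Player-controlled flying pawn that constantly moves forward along its facing, spins two propellers and fires rockets.
; Pitch and Roll axes rotate the actor locally, scaled by frame time, and a FlipFlop alternates BP_Rocket spawns between left and right arrows.
; Holding Boost adds an offset to the FloatingPawnMovement max speed, restored on release.
; An older two-second timed boost remains in the graph but is disconnected.
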(event `self.ReceiveBeginPlay`
  ; MaxSpeed 설정
  (`self.InitMaxSpeed`))

(event `self.ReceiveTick`
  (params (DeltaSeconds :type "Float (single-precision)"))
  ; 전방이동
  (`self.AddMovementInput` (`self.GetActorForwardVector`))
  (`|ExecutionSequence`
    (:`then_0`
      ; 프로펠러 회전
      (`self.RotatePropeller` (`self.LeftPropeller`)))
    (:`then_1`
      (`self.RotatePropeller` (`self.RightPropeller`)))))

(event `InputAxis|Pitch`
  (params (AxisValue :type "Float (single-precision)"))
  ; Pitch
  (`self.K2_AddActorLocalRotation` (`KismetMathLibrary.MakeRotator` 0.0 (* AxisValue (`GameplayStatics.GetWorldDeltaSeconds`) (`self.PichRollSpeed`)))))

(event `InputAxis|Roll`
  (params (AxisValue :type "Float (single-precision)"))
  ; Roll
  (`self.K2_AddActorLocalRotation` (`KismetMathLibrary.MakeRotator` (* AxisValue (`GameplayStatics.GetWorldDeltaSeconds`) (`self.PichRollSpeed`)))))

(event `InputAction|Fire`
  (params (Key :type "Key Structure"))
  ; 로켓 발사
  (:`Pressed`
    (`/Engine/EditorBlueprintResources/StandardMacros.FlipFlop`
      (:`A`
        (`self.SpawnRocket` (`self.LeftArrow`)))
      (:`B`
        (`self.SpawnRocket` (`self.RightArrow`))))))

(event `InputAction|Boost`
  (params (Key :type "Key Structure"))
  ; Boost -> 한번 누르면 2초동안 속도 빨라짐
)

(event `CustomEvent`
  ; Boost -> 한번 누르면 2초동안 속도 빨라짐
  ;; 스피드 되돌리기
  (`self.InitMaxSpeed`)
  (set `self.bIsBoosting` false))

(event `InputAction|Boost`
  (params (Key :type "Key Structure"))
  ; Boost 누를 때만 빨리가는 로직으로
  (:`Pressed`
    (`self.SetBoostSpeed`))
  (:`Released`
    (`self.InitMaxSpeed`)))

(fn `InitMaxSpeed`
  (set `FloatingPawnMovement.MaxSpeed` (`self.MaxSpeed`) (`self.FloatingPawnMovement`)))

(fn `RotatePropeller`
  (params (Propeller :type "SceneComponent Object Reference"))
  (`SceneComponent.K2_AddLocalRotation` Propeller (`KismetMathLibrary.MakeRotator` (* (`GameplayStatics.GetWorldDeltaSeconds`) (`self.RotationSpeed`))) false false)
  (return))

(fn `SetBoostSpeed`
  (set `FloatingPawnMovement.MaxSpeed` (+ (`self.MaxSpeed`) (`self.BoostSpeedOffset`)) (`self.FloatingPawnMovement`)))

(fn `SpawnRocket`
  (params (RocketLocation :type "SceneComponent Object Reference"))
  (`|SpawnActorFromClass` "/Game/Blueprints/BP_Rocket.BP_Rocket_C" (`SceneComponent.K2_GetComponentToWorld` RocketLocation) "AdjustIfPossibleButAlwaysSpawn" "MultiplyWithRoot" null null))

(fn `UserConstructionScript`)