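; BP_Target is a damageable target actor whose destruction clears the game.
; On AnyDamage, CalculateHP subtracts the damage from HP and reports whether HP has reached zero or below.
; When it has, the target destroys itself, casts the game mode to BP_Gamemode and calls GameClear.
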(event `self.ReceiveAnyDamage`
  (params (Damage :type "Float (single-precision)") (DamageType :type "DamageType Object Reference") (InstigatedBy :type "Controller Object Reference") (DamageCauser :type "Actor Object Reference"))
  (bind _output_get (set `self.HP` (- (`self.HP`) Damage)))
  (if (<= _output_get 0.0)
    (`self.K2_DestroyActor`)
    (bind _asbp_gamemode (cast `/Game/Blueprints/BP_Gamemode` (`GameplayStatics.GetGameMode`)))
    (`/Game/Blueprints/BP_Gamemode.GameClear` _asbp_gamemode)))

(fn `UserConstructionScript`)