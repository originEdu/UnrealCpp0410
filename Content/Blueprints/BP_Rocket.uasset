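; BP_Rocket is a short-lived rocket projectile that damages whatever non-player actor it overlaps.
; On BeginPlay it sets a brief lifespan so missed shots clean themselves up.
; On overlap with an actor not tagged Player, it spawns a Niagara explosion and sound at its location, applies fixed damage credited to player controller 0, then destroys itself.
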(event `self.ReceiveBeginPlay`
  (`self.SetLifeSpan` 3.0))

(event `self.ReceiveActorBeginOverlap`
  (params (OtherActor :type "Actor Object Reference"))
  (bind _returnvalue (`self.K2_GetActorLocation`))
  (if (not (`self.ActorHasTag` OtherActor "Player"))
    ; 이펙트 생성
    (`NiagaraFunctionLibrary.SpawnSystemAtLocation` "/Niagara/DefaultAssets/Templates/Systems/SimpleExplosion.SimpleExplosion" _returnvalue)
    ; 사운드 생성
    (`GameplayStatics.SpawnSoundAtLocation` "/Game/Sound/MS_Explosion.MS_Explosion" _returnvalue (struct) 1.0 1.0 0.0 null null)
    ; 데미지 입히기
    (`GameplayStatics.ApplyDamage` OtherActor 10.0 (`GameplayStatics.GetPlayerController` 0) self)
    (`self.K2_DestroyActor`)))

(fn `UserConstructionScript`)